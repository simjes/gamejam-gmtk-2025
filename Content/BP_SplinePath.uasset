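; Spline path actor that renders a spline as a chain of spline meshes, hidden at BeginPlay.
; The construction script adds a spline mesh component per spline point, spanning it to the next index, and stores each in SplineMeshes.
; Every segment takes its start tangent from point 0, while end tangents follow the next index.
; The DrawSplines event shows or hides all stored meshes.
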(event Custom|DrawSplines
  (params (ShouldDraw :type Boolean))
  (for _array_element (Variables|Default|GetSplineMeshes)
    (Rendering|SetVisibility _array_element ShouldDraw false)))

(event EventBeginPlay
  (for _array_element (Variables|Default|GetSplineMeshes)
    (Rendering|SetVisibility _array_element false false)))

(event Collision|EventActorBeginOverlap
  (params (OtherActor :type Actor%20Object%20Reference)))

(event EventTick
  (params (DeltaSeconds :type Float%20%28single-precision%29)))

(fn ConstructionScript
  (bind _spline (Variables|Default|GetSpline))
  (Utilities|Array|Clear (Variables|Default|GetSplineMeshes))
  (for _index (range 0 (- (Spline|GetNumberOfSplinePoints (Variables|Default|GetSpline)) 1))
    (bind _returnvalue (AddComponent|AddSplineMeshComponent false))
    (SplineMesh|SetForwardAxis _returnvalue "X" true)
    (SplineMesh|SetStartandEnd _returnvalue (Spline|GetLocationatSplinePoint _spline _index "Local") (Spline|GetTangentatSplinePoint _spline 0 "Local") (Spline|GetLocationatSplinePoint _spline (+ _index 1) "Local") (Spline|GetTangentatSplinePoint _spline (+ _index 1) "Local") true :!class /Script/Engine.SplineMeshComponent)
    (Utilities|Array|Add (Variables|Default|GetSplineMeshes) _returnvalue)))